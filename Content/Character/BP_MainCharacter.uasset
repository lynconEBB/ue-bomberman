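; BP_MainCharacter is the main character Blueprint, handling player movement through Enhanced Input.
; BeginPlay adds IMC_Default to the local player's input subsystem.
; IA_Move drives movement input along fixed world X and Y axes, with Y negated, and stores the raw input in Directionality.
; The action's start and completion toggle the IsMoving flag.
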(event Input|EnhancedActionEvents|EnhancedInputActionIA_Move
  (params (ActionValue :type Vector%202D%20Structure) (ElapsedSeconds :type Float%20%28double-precision%29) (TriggeredSeconds :type Float%20%28double-precision%29) (InputAction :type Input%20Action%20Object%20Reference :default "/Game/Character/Input/IA_Move.IA_Move"))
  (:Triggered
    (Pawn|Input|AddMovementInput (Math|Vector|MakeVector (.x ActionValue) 0.0 0.0) 1.0 false)
    (Pawn|Input|AddMovementInput (Math|Vector|MakeVector 0.0 (* (.y ActionValue) -1.0) 0.0) 1.0 false)
    (Variables|Default|SetDirectionality (Math|Vector2D|MakeVector2D (.x ActionValue) (.y ActionValue))))
  (:Started
    (Variables|Default|SetbIsMoving true))
  (:Completed
    (Variables|Default|SetbIsMoving false)))

(event EventBeginPlay
  (bind _returnvalue (Pawn|GetController))
  (bind _asplayer_controller (Utilities|Casting|CastToPlayerController _returnvalue))
  (bind _returnvalue_2 (PlayerController|LocalPlayerSubsystems|GetEnhancedInputLocalPlayerSubsystem _asplayer_controller))
  (Utilities|IsValid _returnvalue_2
    (:Is%20Valid
      (Input|AddMappingContext _returnvalue_2 "/Game/Character/Input/IMC_Default.IMC_Default" 0 "(bIgnoreAllPressedKeysUntilRelease=True,bForceImmediately=False)"))))

(fn ConstructionScript)